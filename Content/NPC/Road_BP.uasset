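; Spline-based road actor that supplies path points in world space, likely for NPC navigation.
; GetNextPoint converts a target distance along the spline into a location, flagging EndReached when the distance falls outside the spline.
; GetClosestPoint steps along the spline at coarse fixed intervals, returning the sampled point nearest a given location and its spline distance.
; The event graph and construction script are empty, so the actor only answers queries.
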(event EventBeginPlay)

(event Collision|EventActorBeginOverlap
  (params (OtherActor :type Actor%20Object%20Reference)))

(event EventTick
  (params (DeltaSeconds :type Float%20%28single-precision%29)))

(fn ConstructionScript)

(fn GetNextPoint
  (params (TargetDistance :type Float%20%28single-precision%29))
  (bind _spline (Variables|Default|GetSpline))
  (if (and (> TargetDistance 0.0) (< TargetDistance (Spline|GetSplineLength _spline)))
    (return false (Spline|GetLocationatDistanceAlongSpline _spline TargetDistance "World"))
    (else
      (return true "0, 0, 0"))))

(fn GetClosestPoint
  (params (Location :type Vector))
  (bind _spline (Variables|Default|GetSpline))
  (if (> (Spline|GetSplineLength _spline) (LocalVariables|GetDistance)) :!label _label
    (if (> (LocalVariables|GetMinDistance) (Math|Vector|Distance(Vector) Location (Spline|GetLocationatDistanceAlongSpline _spline (LocalVariables|GetDistance) "World")))
      (LocalVariables|SetMinDistance (Math|Vector|Distance(Vector) Location (Spline|GetLocationatDistanceAlongSpline _spline (LocalVariables|GetDistance) "World")))
      (LocalVariables|SetClosest_Point (Spline|GetLocationatDistanceAlongSpline _spline (LocalVariables|GetDistance) "World"))
      (LocalVariables|SetClosest_SplineLength (LocalVariables|GetDistance)))
    (LocalVariables|SetDistance (+ (LocalVariables|GetDistance) 5e+02))
    (goto _label)
    (else
      (return (LocalVariables|GetClosest_Point) (LocalVariables|GetClosest_SplineLength)))))